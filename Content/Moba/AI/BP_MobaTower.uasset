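; BP_MobaTower is the MOBA defense tower Blueprint, which shows its health bar to players on the tower's team.
; On team change, it calls the parent, then searches the PlayerArray for the local player's state.
; A matching team makes BPHealthBar visible and friendly; otherwise the bar is hidden and marked non-friendly.
; Its Destroyed event only calls StackTrace.
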(event `self.OnTeamChanged`
  (bind _bp_healthbar (`self.BP_HealthBar`))
  ;[1 1 1] 防御塔对友军显示血量
  (`parent.OnTeamChanged`)
  (for _array_element (`GameStateBase.PlayerArray` (`GameplayStatics.GetGameState`))
    (bind _asbp_moba_player_state (cast `/Game/Moba/BluePrints/BP_MobaPlayerState` _array_element))
    (bind _returnvalue (`FPSHeroPlayerStateBase.GetPlayerController` _asbp_moba_player_state))
    (`/Engine/EditorBlueprintResources/StandardMacros.IsValid` _returnvalue
      (:`Is Valid`
        (if (`Controller.IsLocalController` _returnvalue)
          (if (== (`self.GetTeam`) (`FPSHeroPlayerStateBase.GetTeam` _asbp_moba_player_state))
            (`SceneComponent.SetVisibility` _bp_healthbar true false)
            (`/Game/Moba/BluePrints/BP_HealthBar.Set Friendly` _bp_healthbar true)
            (break)
            (else
              (`SceneComponent.SetVisibility` _bp_healthbar false false)
              (`/Game/Moba/BluePrints/BP_HealthBar.Set Friendly` _bp_healthbar false)
              (break))))))))

(event `self.ReceiveDestroyed`
  (`KismetSystemLibrary.StackTrace`))

(fn `UserConstructionScript`
  (`parent.UserConstructionScript`))