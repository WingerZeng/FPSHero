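; AI controller for MOBA defense towers that limits targeting to enemy minions and heroes.
; ShouldAimActor rejects other towers, then accepts a character only if its team differs from the controlled pawn's and is neither none nor neutral.
; Team values are converted to the team enum through BP_MobaGameMode, reached via the GameState's authority game mode.
; The event graph and construction script add no logic of their own.
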(fn `Should Aim Actor`
  (params (Character :type "FPSHeroCharacter Object Reference"))
  (returns (bShouldAim :type Boolean))
  ;[1 1 1] 防御塔只会打小兵和英雄
  (cast `/Game/Moba/AI/BP_MobaTower` Character
    (:`then`
      (return false))
    (:`CastFailed`
      (bind _asbp_moba_game_mode (cast `/Game/Moba/BluePrints/BP_MobaGameMode` (`GameStateBase.AuthorityGameMode` (`GameplayStatics.GetGameState`))))
      (bind _asfpshero_character (cast `FPSHeroCharacter` (`self.K2_GetPawn`)))
      (bind _teamenum (`/Game/Moba/BluePrints/BP_MobaGameMode.Cast Int To ETeam` _asbp_moba_game_mode (`FPSHeroCharacter.GetTeam` Character)))
      (if (and (`|EnumInequality` (`/Game/Moba/BluePrints/BP_MobaGameMode.Cast Int To ETeam` _asbp_moba_game_mode (`FPSHeroCharacter.GetTeam` _asfpshero_character)) _teamenum) (`|EnumInequality` _teamenum "TEAM_NONE") (`|EnumInequality` _teamenum "TEAM_NEUTRAL"))
        (return true)
        (else
          (return false))))))

(fn `UserConstructionScript`
  (`parent.UserConstructionScript`))