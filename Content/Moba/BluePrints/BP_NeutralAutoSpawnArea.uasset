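; BP_NeutralAutoSpawnArea is a MOBA spawn area that places a neutral creature inside itself after a delay.
; BeginSpawn sets a one-shot timer for SpawnSingle, which proceeds only if the alive count is at or above MaxAliveCnt.
; It retries collision-adjusted spawns at parent-provided locations with random yaw until one succeeds.
; Each neutral receives this area as its patrol area and leaves AliveNeutrals when destroyed.
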(event `BeginSpawn`
  (`KismetSystemLibrary.K2_SetTimerDelegate` (delegate `SpawnSingle`) (`self.SpawnInterval`)))

(event `SpawnSingle`
  (bind _spawningneutral (`self.SpawningNeutral`))
  (if (>= (`KismetArrayLibrary.Array_Length` (`self.AliveNeutrals`)) (`self.MaxAliveCnt`))
    (set `self.SpawningNeutral` null)
    ;[1 1 1] 尝试在区域内随机位置生成中立生物直到成功
    (while (not (`KismetSystemLibrary.IsValid` (`self.SpawningNeutral`)))
      (bind _spawnlocation (`self.GetSpawnLocation`))
      (bind _returnvalue (`|SpawnActorFromClass` (`self.NeutralType`) (`KismetMathLibrary.MakeTransform` _spawnlocation (`KismetMathLibrary.MakeRotator` 0.0 0.0 (`KismetMathLibrary.RandomFloatInRange` 0.0 360.0))) "AdjustIfPossibleButDontSpawnIfColliding" "OverrideRootScale" null null))
      (set `self.SpawningNeutral` _returnvalue))
    (add `Actor.OnDestroyed` (`self.SpawningNeutral`) (delegate `OnNeutralDestroyed`))
    (`KismetArrayLibrary.Array_Add` (`self.AliveNeutrals`) _spawningneutral)
    (`/Game/Moba/AI/BP_MobaNeutral.SetupPatrolArea` _spawningneutral self)))

(event `OnNeutralDestroyed`
  (params (DestroyedActor :type "Actor Object Reference"))
  ;[1 1 1] 中立对象被Destroy时需要移除
  (bind _asbp_moba_neutral (cast `/Game/Moba/AI/BP_MobaNeutral` DestroyedActor))
  (`KismetArrayLibrary.Array_RemoveItem` (`self.AliveNeutrals`) _asbp_moba_neutral))

(fn `GetSpawnLocation`
  (returns (SpawnLocation :type "Vector Structure"))
  (bind _spawnlocation (`parent.GetSpawnLocation`))
  (return _spawnlocation))

(fn `UserConstructionScript`
  (`parent.UserConstructionScript`))