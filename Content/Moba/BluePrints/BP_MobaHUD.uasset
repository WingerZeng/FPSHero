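; BP_MobaHUD is the Moba HUD class that creates the main UMG widget on BeginPlay and adds it to the viewport.
; Its CharacterUpdate event reads the owning player character's health and current weapon ammo, plus money from the player state.
; It pushes those values into the widget's HP, ammo and money displays, skipping ammo when no weapon is valid.
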(event `self.ReceiveBeginPlay`
  (bind _returnvalue (`|CreateWidget` "/Game/Moba/UMG/BP_MobaMainUMG.BP_MobaMainUMG_C"))
  (bind _output_get (set `self.MainUMG` _returnvalue))
  (`UserWidget.AddToViewport` _output_get 0))

(event `self.CharacterUpdate`
  (bind _mainumg (`self.MainUMG`))
  (`/Engine/EditorBlueprintResources/StandardMacros.IsValid` (`self.MainUMG`)
    (:`Is Valid`
      (bind _asbp_moba_player_character (cast `/Game/Moba/BluePrints/BP_MobaPlayerCharacter` (`self.GetOwningPawn`)))
      (bind _returnvalue (`FPSHeroCharacter.GetHealth` _asbp_moba_player_character))
      (bind _returnvalue_2 (`FPSHeroCharacter.GetMaxHealth` _asbp_moba_player_character))
      (`/Game/Moba/UMG/BP_MobaMainUMG.SetHP` _mainumg (`KismetMathLibrary.FTrunc` _returnvalue) (`KismetMathLibrary.FTrunc` _returnvalue_2))
      (bind _returnvalue_3 (`FPSHeroCharacter.GetCurrentWeapon` _asbp_moba_player_character))
      (`/Engine/EditorBlueprintResources/StandardMacros.IsValid` _returnvalue_3
        (:`Is Valid`
          (`/Game/Moba/UMG/BP_MobaMainUMG.SetAmmo` _mainumg (`FPSHeroWeaponBase.GetAmmo` _returnvalue_3) (`FPSHeroWeaponBase.GetTotalAmmo` _returnvalue_3)))
        (:`Is Not Valid`
          _))
      (bind _asbp_moba_player_state (cast `/Game/Moba/BluePrints/BP_MobaPlayerState` (`Pawn.PlayerState` _asbp_moba_player_character)))
      (`/Game/Moba/UMG/BP_MobaMainUMG.SetMoney` _mainumg (`FPSHeroPlayerStateBase.GetMoney` _asbp_moba_player_state)))))

(fn `UserConstructionScript`)