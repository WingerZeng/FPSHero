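; BP_SpawnArea is a box-shaped spawn area that supplies random navigable spawn locations within its bounds.
; GetSpawnLocation samples navigable points in the box's bounding sphere and rejects any outside the transformed box.
; It retries up to MaxLoops and falls back to the box bounds' center when no valid point is found.
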(fn `GetSpawnLocation`
  (returns (SpawnLocation :type "Vector Structure"))
  (locals (bIsFound :type Boolean :default false) (TempLocation :type "Vector Structure" :default (0.0 0.0 0.0)) (Loops :type Integer))
  (bind _box (`self.Box`))
  (bind (_origin _boxextent _sphereradius) (`KismetSystemLibrary.GetComponentBounds` (`self.Box`)))
  (while (and (not (`local.bIsFound`)) (< (`local.Loops`) (`self.MaxLoops`)))
    (bind (_randomlocation _returnvalue) (`NavigationSystemV1.K2_GetRandomLocationInNavigableRadius` _origin _sphereradius null null))
    (set `local.TempLocation` _randomlocation)
    (`/Engine/EditorBlueprintResources/StandardMacros.IncrementInt` (`local.Loops`)
      (:`  `
        (set `local.bIsFound` (and _returnvalue (`KismetMathLibrary.IsPointInBoxWithTransform` _randomlocation (`SceneComponent.K2_GetComponentToWorld` _box) (`BoxComponent.BoxExtent` _box)))))))
  (if (`local.bIsFound`)
    (return (`local.TempLocation`))
    (else
      (return _origin))))

(fn `UserConstructionScript`)