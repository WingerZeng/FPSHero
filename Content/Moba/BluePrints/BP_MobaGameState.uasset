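; BP_MobaGameState is the MOBA game state Blueprint that provides team coloring for characters.
; ColorCharacter looks up the character's team in the TeamColors map and does nothing if no entry exists.
; It creates dynamic mannequin material instances for the body and chest logo on Mesh, and the body only on Mesh1P.
; Each instance receives the team color through its BodyColor parameter.
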(fn `ColorCharacter`
  (params (Character :type "FPSHeroCharacter Object Reference"))
  (bind _mesh (`Character.Mesh` Character))
  (bind (_value _returnvalue) (`BlueprintMapLibrary.Map_Find` (`self.TeamColors`) (`FPSHeroCharacter.GetETeam` Character)))
  (if _returnvalue
    (`|ExecutionSequence`
      (:`then_0`
        (bind _returnvalue_2 (`PrimitiveComponent.CreateDynamicMaterialInstance` _mesh 0 "/Game/Animations/UE4_Mannequin/Materials/M_UE4Man_Body.M_UE4Man_Body" "None"))
        (`MaterialInstanceDynamic.SetVectorParameterValue` _returnvalue_2 "BodyColor" _value)
        (bind _returnvalue_3 (`PrimitiveComponent.CreateDynamicMaterialInstance` _mesh 1 "/Game/Animations/UE4_Mannequin/Materials/M_UE4Man_ChestLogo.M_UE4Man_ChestLogo" "None"))
        (`MaterialInstanceDynamic.SetVectorParameterValue` _returnvalue_3 "BodyColor" _value))
      (:`then_1`
        (bind _returnvalue_4 (`PrimitiveComponent.CreateDynamicMaterialInstance` (`FPSHeroCharacter.Mesh1P` Character) 0 "/Game/Animations/UE4_Mannequin/Materials/M_UE4Man_Body.M_UE4Man_Body" "None"))
        (`MaterialInstanceDynamic.SetVectorParameterValue` _returnvalue_4 "BodyColor" _value)))))

(fn `UserConstructionScript`)