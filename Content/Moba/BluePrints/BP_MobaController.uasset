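; BP_MobaController is a controller for the MOBA game that handles damage feedback and store input.
; When it instigates positive damage, it shows the damaged actor's health bar for a configurable time, fetching the bar through HealthBarInterface.
; The Store input action, on the local controller only, calls SwitchStore on BP_MobaHUD.
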(event `self.ReceiveInstigatedAnyDamage`
  (params (Damage :type "Float (single-precision)") (DamageType :type "DamageType Object Reference") (DamagedActor :type "Actor Object Reference") (DamageCauser :type "Actor Object Reference"))
  (if (> Damage 0.0)
    (`self.ShowHealthBar` DamagedActor)))

(event `ShowHealthBar`
  (params (Actor :type "Actor Object Reference"))
  (bind _ashealth_bar_interface (cast `/Game/Moba/BluePrints/HealthBarInterface` Actor))
  (bind _healthbar (`/Game/Moba/BluePrints/HealthBarInterface.GetHealthBar` _ashealth_bar_interface))
  (`/Game/Moba/BluePrints/BP_HealthBar.ShowForTime` _healthbar (`self.HealthBarShowTime`)))

(event `InputAction|Store`
  (params (Key :type "Key Structure"))
  (:`Pressed`
    (if (`self.IsLocalController`)
      (bind _asbp_moba_hud (cast `/Game/Moba/BluePrints/BP_MobaHUD` (`self.GetHUD`)))
      (`/Game/Moba/BluePrints/BP_MobaHUD.SwitchStore` _asbp_moba_hud))))

(fn `UserConstructionScript`)