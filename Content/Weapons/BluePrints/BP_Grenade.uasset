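; Grenade weapon Blueprint that animates the prepare and release phases of a throw on the owning character's current mesh.
; StartPrepare plays ThrowMontage and calls ReadyToThrow on the ready notify, while StartRelease plays it from the throw section and calls ThrowOut on the out notify.
; IsMontagePlaying tracks playback.
; When release ends, is interrupted or hits any notify end, the authority removes the weapon from the owner's slot and clears that flag.
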(event `self.StartPrepare`
  (bind _returnvalue (`self.GetOwnerCharacter`))
  (bind _returnvalue_2 (`FPSHeroCharacter.GetCurrentMesh` _returnvalue))
  (bind _notifyname (`|PlayMontage` _returnvalue_2 (`self.ThrowMontage`) 1.0 0.0 "None")
    (:`then`
      (set `self.IsMontagePlaying` true))
    (:`OnCompleted`
      (set `self.IsMontagePlaying` false :!label _label))
    (:`OnBlendOut`
      (goto _label))
    (:`OnInterrupted`
      (goto _label))
    (:`OnNotifyBegin`
      (if (== _notifyname (`self.ThrowReadyNotifyName`))
        (`self.ReadyToThrow`)))))

(event `self.StartRelease`
  (bind _returnvalue (`self.GetOwnerCharacter`))
  (bind _returnvalue_2 (`FPSHeroCharacter.GetCurrentMesh` _returnvalue))
  (bind _notifyname (`|PlayMontage` _returnvalue_2 (`self.ThrowMontage`) 1.0 0.0 (`self.ThrowSectionName`))
    (:`then`
      (set `self.IsMontagePlaying` true))
    (:`OnCompleted`
      (bind _returnvalue_3 (`self.GetOwnerCharacter` :!label _label_2))
      (if (`|EnumEquality` (`self.GetLocalRole` _returnvalue_3) "ROLE_Authority")
        (`FPSHeroCharacter.RemoveWeapon` _returnvalue_3 (`self.SlotInOwner`))
        (set `self.IsMontagePlaying` false)))
    (:`OnBlendOut`
      (goto _label_2))
    (:`OnInterrupted`
      (goto _label_2))
    (:`OnNotifyBegin`
      (if (== _notifyname (`self.ThrowOutNotifyName`))
        (`self.ThrowOut`)))
    (:`OnNotifyEnd`
      (goto _label_2))))

(fn `UserConstructionScript`)