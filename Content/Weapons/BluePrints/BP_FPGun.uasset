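; BP_FPGun is a first-person gun Blueprint whose spotlight follows the owning character's aim while the weapon is active.
; Each Tick it sets the SpotLight's world rotation to the owner's view rotation and shows the light.
; The light is hidden when the owner is invalid or the weapon is inactive, with visibility changed only when it differs from the wanted state.
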(event `self.ReceiveTick`
  (params (DeltaSeconds :type "Float (single-precision)"))
  (bind _spotlight (`self.SpotLight`))
  (bind _spotlight_2 (`self.SpotLight`))
  (bind _returnvalue (`SceneComponent.IsVisible` _spotlight_2))
  (bind _returnvalue_2 (`self.GetOwnerCharacter`))
  (if (and (`KismetSystemLibrary.IsValid` _returnvalue_2) (`self.bIsWeaponActive`))
    (`SceneComponent.K2_SetWorldRotation` _spotlight (`FPSHeroCharacter.GetCharacterViewRotation` _returnvalue_2) false false)
    (if (not _returnvalue)
      (`SceneComponent.SetVisibility` _spotlight true false))
    (elif _returnvalue
      (`SceneComponent.SetVisibility` _spotlight_2 false false))))

(fn `UserConstructionScript`)