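; BP_IntTotalWidget is an actor Blueprint that displays an integer count against a total as "Value/Total" on its IntValue text.
; SetValue stores the new value and rebuilds the text, and BeginPlay calls it with the stored value to show the initial state.
; SetTotalCnt only stores the total, so the displayed text picks it up on the next SetValue call.
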(event `self.ReceiveBeginPlay`
  (`self.SetValue` (`self.value`)))

(event `SetValue`
  (params (value :type Integer))
  (bind _output_get (set `self.value` value))
  (`TextRenderComponent.K2_SetText` (`self.IntValue`) (`KismetTextLibrary.Conv_StringToText` (`KismetStringLibrary.Concat_StrStr` (`KismetStringLibrary.Conv_IntToString` _output_get) "/" (`KismetStringLibrary.Conv_IntToString` (`self.TotalCnt`))))))

(event `SetTotalCnt`
  (params (`Total Count` :type Integer))
  (set `self.TotalCnt` `Total Count`))

(fn `UserConstructionScript`)