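; BP_WeaponButton is an in-world button that displays a weapon and gives it to the hero character when hit.
; On BeginPlay it spawns an instance of WeaponClass and snaps it to its Scene component before running the parent's BeginPlay.
; OnHit finds the FPSHeroCharacter, has it grip a weapon of that class, then switches it to that weapon type's slot.
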(event `self.OnHit`
  (bind _weaponclass (`self.WeaponClass`))
  (bind _returnvalue (`GameplayStatics.GetActorOfClass` "/Script/FPSHero.FPSHeroCharacter"))
  (`FPSHeroCharacter.GripWeapon` _returnvalue _weaponclass)
  (bind _returnvalue_2 (`FPSHeroCharacter.GetWeaponTypeSlot` _returnvalue _weaponclass))
  (`FPSHeroCharacter.SwitchToWeaponSlot` _returnvalue _returnvalue_2))

(event `self.ReceiveBeginPlay`
  (bind _returnvalue (`|SpawnActorFromClass` (`self.WeaponClass`) (`KismetMathLibrary.MakeTransform` (0.0 0.0 0.0)) "AlwaysSpawn" "OverrideRootScale" null null))
  (bind _output_get (set `self.WeaponInstance` _returnvalue))
  (`self.K2_AttachToComponent` _output_get (`self.Scene`) "None" "SnapToTarget" "SnapToTarget" "KeepRelative" true)
  (`parent.ReceiveBeginPlay`))

(fn `UserConstructionScript`
  (`parent.UserConstructionScript`))