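; Game mode that switches a training session between preparing and running states and shows the success or failure result.
; Each state toggles visibility, collision and tick on actors tagged PreparingWidget or StartingWidget, and starting also zeroes the TargetRemainWidget counters.
; Results restyle every BP_ScrollText, then after a five-second delay restore the preparing actors and reset the text.
; BeginPlay disables VSync and caps the frame rate at 144.
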(event `self.ReceiveBeginPlay`
  (bind _returnvalue (`GameUserSettings.GetGameUserSettings`))
  (`GameUserSettings.SetVSyncEnabled` _returnvalue false)
  (`KismetSystemLibrary.ExecuteConsoleCommand` "t.maxfps 144" null))

(event `Training Successful`
  (`self.DIsableBeginingActor` true)
  (bind _outactors (`GameplayStatics.GetAllActorsOfClass` "/Game/BluePrints/BP_ScrollText.BP_ScrollText_C"))
  (for _array_element _outactors
    (`/Game/BluePrints/BP_ScrollText.Set Text` _array_element "/Game/BluePrints/BP_SuccessfulText.BP_SuccessfulText_C" (make `Color` 0 255 255 255) 200.0 300.0)
    (`KismetSystemLibrary.Delay` 5.0 :!label _label)
    (`self.Disable Preparing Actor` false)
    (bind _outactors_2 (`GameplayStatics.GetAllActorsOfClass` "/Game/BluePrints/BP_ScrollText.BP_ScrollText_C"))
    (for _array_element_2 _outactors_2
      (`/Game/BluePrints/BP_ScrollText.Set Text` :`self` _array_element_2 :`Spacing` 200.0 :`Speed` 200.0))))

(event `Training Failed`
  (`self.DIsableBeginingActor` true)
  (bind _outactors (`GameplayStatics.GetAllActorsOfClass` "/Game/BluePrints/BP_ScrollText.BP_ScrollText_C"))
  (for _array_element _outactors
    (`/Game/BluePrints/BP_ScrollText.Set Text` _array_element "/Game/BluePrints/BP_FailedText.BP_FailedText_C" (make `Color` 0 0 100 255) 150.0 300.0)
    (goto _label)))

(event `Begin Training`
  (`self.Disable Preparing Actor` true)
  (`self.DIsableBeginingActor` false)
  (bind _outactors (`GameplayStatics.GetAllActorsWithTag` "TargetRemainWidget"))
  (for _array_element _outactors
    (bind _asbp_int_total_widget (cast `/Game/BluePrints/BP_IntTotalWidget` _array_element))
    (`/Game/BluePrints/BP_IntTotalWidget.SetTotalCnt` _asbp_int_total_widget 0)))

(event `Stop Trainging`
  (`self.DIsableBeginingActor` true)
  (`self.Disable Preparing Actor` false))

(fn `Disable Preparing Actor`
  (params (`Is Disabled` :type Boolean))
  (bind _outactors (`GameplayStatics.GetAllActorsWithTag` "PreparingWidget"))
  (for _array_element _outactors
    (`self.Set Actor Disabled` `Is Disabled` _array_element)))

(fn `DIsableBeginingActor`
  (params (isDisabled :type Boolean))
  (bind _outactors (`GameplayStatics.GetAllActorsWithTag` "StartingWidget"))
  (for _array_element _outactors
    (`self.Set Actor Disabled` isDisabled _array_element)))

(fn `Set Actor Disabled`
  (params (IsDisabled :type Boolean) (actor :type "Actor Object Reference"))
  (bind _returnvalue (not IsDisabled))
  (`self.SetActorHiddenInGame` actor IsDisabled)
  (`self.SetActorEnableCollision` actor _returnvalue)
  (`self.SetActorTickEnabled` actor _returnvalue))

(fn `UserConstructionScript`)