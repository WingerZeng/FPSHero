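; Scrolling text actor that streams repeated copies of a text actor class through a Box volume, like a marquee.
; Each tick moves the copies along MoveOrient's X axis, destroys leading ones that leave the Box and spawns spaced replacements behind until it is filled.
; A shared dynamic material receives the Box bounds and color.
; SetText changes class, color, spacing and speed; an invalid class clears all copies.
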(event `self.ReceiveBeginPlay`
  (`self.Init Material`))

(event `self.ReceiveTick`
  (params (DeltaSeconds :type "Float (single-precision)"))
  (bind _textobjects (`self.TextObjects`))
  (set `self.Delta` DeltaSeconds)
  (if (`KismetSystemLibrary.IsValidClass` (`self.TextType`))
    (if (== (`KismetArrayLibrary.Array_Length` (`self.TextObjects`)) 0)
      (`self.Add Single Text` (`self.K2_GetActorLocation`))
      (`self.Fill Text Objects`)
      (else
        (`self.Update Text Position`)
        (`self.Remove Expire Text`)
        (`self.Fill Text Objects`)))
    (else
      (for _array_element _textobjects
        (`self.K2_DestroyActor` _array_element))
      (`KismetArrayLibrary.Array_Clear` _textobjects))))

(event `Set Text`
  (params (`Text Render Type` :type "TextRenderActor Class Reference") (Color :type "Color Structure") (Spacing :type "Float (double-precision)") (Speed :type "Float (double-precision)" :default 0.0))
  (set `self.TextType` `Text Render Type`)
  (set `self.BaseColor` Color)
  (set `self.Spacing` Spacing)
  (set `self.Speed` Speed)
  (`self.Init Material`))

(fn `Add Single Text`
  (params (Location :type "Vector Structure"))
  (returns (`Text Actor` :type "TextRenderActor Object Reference"))
  (bind _returnvalue (`|SpawnActorFromClass` (`self.TextType`) (`KismetMathLibrary.MakeTransform` Location) "AlwaysSpawn" "OverrideRootScale" self null))
  (`self.K2_AttachToComponent` _returnvalue (`self.DefaultSceneRoot`) "None" "KeepWorld" "KeepRelative" "KeepWorld" true)
  (`TextRenderComponent.SetTextMaterial` (`TextRenderActor.TextRender` _returnvalue) (`self.Text Material`))
  (`KismetArrayLibrary.Array_Add` (`self.TextObjects`) _returnvalue)
  (return _returnvalue))

(fn `Destroy Text`
  (params (Index :type Integer))
  (bind _textobjects (`self.TextObjects`))
  (`self.K2_DestroyActor` (`|GetArrayItem` _textobjects Index))
  (`KismetArrayLibrary.Array_Remove` _textobjects Index))

(fn `Fill Text Objects`
  (locals (IsContinue :type Boolean :default true))
  (bind _textobjects (`self.TextObjects`))
  (while (`local.IsContinue`)
    (bind _world_spacing (`self.Get World Spacing`))
    (bind _text_actor (`self.Add Single Text` (+ _world_spacing (`self.K2_GetActorLocation` (`|GetArrayItem` _textobjects (`KismetArrayLibrary.Array_LastIndex` _textobjects))))))
    (bind _output_get (set `local.IsContinue` (`PrimitiveComponent.IsOverlappingActor` (`self.Box`) _text_actor)))
    (if (not _output_get)
      (`self.Destroy Text` (`KismetArrayLibrary.Array_LastIndex` (`self.TextObjects`))))))

(fn `Get World Spacing`
  (returns (`World Spacing` :type "Vector Structure"))
  (bind (_returnvalue_location _returnvalue_rotation) (`KismetMathLibrary.BreakTransform` (`SceneComponent.K2_GetComponentToWorld` (`self.MoveOrient`))))
  (return (* (`KismetMathLibrary.NegateVector` (`KismetMathLibrary.TransformLocation` (`KismetMathLibrary.MakeTransform` (0.0 0.0 0.0) _returnvalue_rotation) (`KismetMathLibrary.MakeVector` 1.0))) (`self.Spacing`))))

(fn `Get World Speed`
  (returns (NewParam :type "Vector Structure"))
  (bind (_returnvalue_location _returnvalue_rotation) (`KismetMathLibrary.BreakTransform` (`SceneComponent.K2_GetComponentToWorld` (`self.MoveOrient`))))
  (return (* (`KismetMathLibrary.TransformLocation` (`KismetMathLibrary.MakeTransform` (0.0 0.0 0.0) _returnvalue_rotation) (`KismetMathLibrary.MakeVector` 1.0)) (`self.Speed`))))

(fn `Init Material`
  (bind (_origin _boxextent) (`KismetSystemLibrary.GetComponentBounds` (`self.Box`)))
  (bind _returnvalue (`KismetMaterialLibrary.CreateDynamicMaterialInstance` "/Game/Materials/ScrollTextMaterialOpaque.ScrollTextMaterialOpaque"))
  (bind _output_get (set `self.Text Material` _returnvalue))
  (`MaterialInstanceDynamic.SetVectorParameterValue` _output_get "NegBound" (`KismetMathLibrary.Conv_VectorToLinearColor` (- _origin _boxextent)))
  (`MaterialInstanceDynamic.SetVectorParameterValue` _output_get "PosBound" (`KismetMathLibrary.Conv_VectorToLinearColor` (+ _origin _boxextent)))
  (`MaterialInstanceDynamic.SetVectorParameterValue` _output_get "Color" (`KismetMathLibrary.Conv_ColorToLinearColor` (`self.BaseColor`))))

(fn `Remove Expire Text`
  (for (_array_element _array_index) (`self.TextObjects`)
    (if (not (`PrimitiveComponent.IsOverlappingActor` (`self.Box`) _array_element))
      (`self.Destroy Text` _array_index)
      (else
        (break)))))

(fn `Update Text Position`
  (for _array_element (`self.TextObjects`)
    (bind _newparam (`self.Get World Speed`))
    (`self.K2_SetActorLocation` _array_element (+ (* _newparam (`self.Delta`)) (`self.K2_GetActorLocation` _array_element)) false false)))

(fn `UserConstructionScript`)