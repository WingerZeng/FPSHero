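; BP_IntSpinBox is an integer spin box with up and down button boxes and a text readout of the current Number.
; Each button hit steps Number by UnitInterval, and ResetNumber refreshes the text, as it does on BeginPlay.
; Increments have no upper limit, while decrements apply only if the result, converted to a byte, is above zero.
; GetNumber exposes the current value to other Blueprints.
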(event `self.ReceiveBeginPlay`
  (`self.ResetNumber` (`self.Number`)))

(event `ResetNumber`
  (params (Number :type Integer))
  (`TextRenderComponent.K2_SetText` (`self.NumberText`) (`KismetTextLibrary.Conv_IntToText` Number)))

(event `self.ButtonBoxUp.OnButtonHit`
  (params (HitComponent :type "PrimitiveComponent Object Reference"))
  (bind _output_get (set `self.Number` (+ (`self.Number`) (`self.UnitInterval`))))
  (`self.ResetNumber` _output_get :!label _label))

(event `self.ButtonBoxDown.OnButtonHit`
  (params (HitComponent :type "PrimitiveComponent Object Reference"))
  (bind _returnvalue (- (`self.Number`) (`self.UnitInterval`)))
  (if (> (`KismetMathLibrary.Conv_IntToByte` _returnvalue) 0)
    (set `self.Number` _returnvalue)
    (goto _label)))

(fn `GetNumber`
  (returns (Number :type Integer))
  (return (`self.Number`)))

(fn `UserConstructionScript`)