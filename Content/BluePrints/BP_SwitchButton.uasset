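; BP_SwitchButton is a toggle button that shows its checked state through the color of a text component.
; Each OnHit flips IsChecked and calls StateChanged, which colors the text red when checked and gray otherwise.
; BeginPlay calls StateChanged once so the text matches the initial IsChecked value.
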(event `self.ReceiveBeginPlay`
  (`self.StateChanged` (`self.IsChecked`)))

(event `StateChanged`
  (params (isChecked :type Boolean))
  (bind _text (`self.Text`))
  (if isChecked
    (`TextRenderComponent.SetTextRenderColor` _text (make `Color` 0 0 255))
    (else
      (`TextRenderComponent.SetTextRenderColor` _text (make `Color` 100 100 100)))))

(event `self.OnHit`
  (bind _output_get (set `self.IsChecked` (not (`self.IsChecked`))))
  (`self.StateChanged` _output_get))

(fn `UserConstructionScript`
  (`parent.UserConstructionScript`))