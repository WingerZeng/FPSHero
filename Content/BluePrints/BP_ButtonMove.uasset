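; BP_ButtonMove is a toggle button that switches the move state held by the game state.
; It overrides StateChanged, calls the parent handler, then casts the game state to BP_GameState and passes the checked value to SetMoveState.
; The trailing branch does nothing, and the "Obstacle: ON/OFF" label updates are disconnected, so they never run.
; The construction script only calls its parent.
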(event `self.StateChanged`
  (params (isChecked :type Boolean))
  (`parent.StateChanged` isChecked)
  (bind _asbp_game_state (cast `/Game/BluePrints/BP_GameState` (`GameplayStatics.GetGameState`)))
  (`/Game/BluePrints/BP_GameState.Set Move State` _asbp_game_state isChecked)
  (if isChecked
    _))

(fn `UserConstructionScript`
  (`parent.UserConstructionScript`))