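; Game state for a timed shooting-style training session in which killed robots count down a target total.
; BeginTraining reads time and target from spin-box actors, and Tick counts down, updates tag-found widget actors and reports success or failure to BP_GameMode.
; It also holds a movement flag and toggles "obscale"-tagged obstacles by offsetting them vertically far away or back.
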(event `self.ReceiveBeginPlay`
  (`self.Stop Training`))

(event `self.ReceiveTick`
  (params (DeltaSeconds :type "Float (single-precision)"))
  (bind _returnvalue (`GameplayStatics.GetGameMode`))
  (if (`self.IsTrainingBegin`)
    (set `self.TimeRemain` (- (`self.TimeRemain`) DeltaSeconds))
    (if (<= (`self.TargetRemain`) 0)
      (bind _asbp_game_mode (cast `/Game/BluePrints/BP_GameMode` _returnvalue))
      (set `self.IsTrainingBegin` false)
      (`/Game/BluePrints/BP_GameMode.Training Successful` _asbp_game_mode)
      (elif (<= (`self.TimeRemain`) 0.0)
        (bind _asbp_game_mode_2 (cast `/Game/BluePrints/BP_GameMode` _returnvalue))
        (set `self.IsTrainingBegin` false)
        (`/Game/BluePrints/BP_GameMode.Training Failed` _asbp_game_mode_2)
        (else
          (bind _outactors (`GameplayStatics.GetAllActorsWithTag` "TargetRemainWidget"))
          (for _array_element _outactors
            (bind _asbp_int_total_widget (cast `/Game/BluePrints/BP_IntTotalWidget` _array_element))
            (`/Game/BluePrints/BP_IntTotalWidget.SetValue` _asbp_int_total_widget (`self.TargetRemain`))
            (bind _outactors_2 (`GameplayStatics.GetAllActorsWithTag` "TimeRemainWidget"))
            (for _array_element_2 _outactors_2
              (bind _asbp_int_widget (cast `/Game/BluePrints/BP_IntWidget` _array_element_2))
              (`/Game/BluePrints/BP_IntWidget.SetValue` _asbp_int_widget (`KismetMathLibrary.FTrunc` (`self.TimeRemain`))))))))))

(event `Set Obstacle State`
  (params (On :type Boolean))
  (bind _returnvalue (`KismetMathLibrary.MakeVector` 0.0 0.0 10000.0))
  (bind _outactors (`GameplayStatics.GetAllActorsWithTag` "obscale"))
  (for _array_element _outactors
    (if On
      (`self.K2_AddActorLocalOffset` _array_element _returnvalue false false)
      (else
        (`self.K2_AddActorLocalOffset` _array_element (`KismetMathLibrary.NegateVector` _returnvalue) false false)))))

(event `Set Move State`
  (params (on :type Boolean))
  (set `self.bMove` on))

(event `Begin Training`
  (bind _returnvalue (`GameplayStatics.GetActorOfClass` "/Game/BluePrints/BP_IntSpinBox_Time.BP_IntSpinBox_Time_C"))
  (bind _number (`/Game/BluePrints/BP_IntSpinBox.GetNumber` _returnvalue))
  (set `self.TimeRemain` (`KismetMathLibrary.Conv_IntToDouble` _number))
  (bind _returnvalue_2 (`GameplayStatics.GetActorOfClass` "/Game/BluePrints/BP_IntSpinBox_Target.BP_IntSpinBox_Target_C"))
  (bind _number_2 (`/Game/BluePrints/BP_IntSpinBox.GetNumber` _returnvalue_2))
  (bind _output_get (set `self.TargetRemain` _number_2))
  (bind _outactors (`GameplayStatics.GetAllActorsWithTag` "TargetRemainWidget"))
  (for _array_element _outactors
    (bind _asbp_int_total_widget (cast `/Game/BluePrints/BP_IntTotalWidget` _array_element))
    (`/Game/BluePrints/BP_IntTotalWidget.SetTotalCnt` _asbp_int_total_widget _output_get)
    (set `self.IsTrainingBegin` true)
    (bind _asbp_game_mode (cast `/Game/BluePrints/BP_GameMode` (`GameplayStatics.GetGameMode`)))
    (`/Game/BluePrints/BP_GameMode.Begin Training` _asbp_game_mode)))

(event `Stop Training`
  (set `self.IsTrainingBegin` false)
  (bind _asbp_game_mode (cast `/Game/BluePrints/BP_GameMode` (`GameplayStatics.GetGameMode`)))
  (`/Game/BluePrints/BP_GameMode.Stop Trainging` _asbp_game_mode))

(event `Kill Robot`
  (if (`self.IsTrainingBegin`)
    (`/Engine/EditorBlueprintResources/StandardMacros.DecrementInt` (`self.TargetRemain`))))

(fn `Can Move`
  (returns (`Can Move` :type Boolean))
  (return (`self.bMove`)))

(fn `UserConstructionScript`)