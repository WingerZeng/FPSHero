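; BP_Target is a robot target character that wanders the level and can be killed by gun and grenade damage.
; Tick starts a new AI move to a random reachable nearby point whenever the previous one ends and BP_GameState allows movement.
; Point and radial damage reduce Health and apply an impulse taken from the gun or grenade damage type.
; At zero Health it reports KillRobot to the game state, enables mesh physics, then destroys itself after a delay.
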(event `self.ReceiveBeginPlay`
  (set `CharacterMovementComponent.MaxWalkSpeed` (`self.WalkSpeed`) (`self.CharacterMovement`)))

(event `Wander`
  (set `self.IsWander` true)
  (`|AIMoveTo` self (`NavigationSystemV1.K2_GetRandomReachablePointInRadius` (`self.K2_GetActorLocation` self) (`self.NaviRadius`) null null) null
    (:`OnSuccess`
      _)
    (:`OnFail`
      _))
  (`KismetSystemLibrary.Delay` 0.2)
  (set `self.IsWander` false))

(event `self.ReceiveTick`
  (params (DeltaSeconds :type "Float (single-precision)"))
  (if (<= (`self.Health`) 0.0)
    (`KismetSystemLibrary.Delay` (`self.DeathDuration`))
    (`self.K2_DestroyActor`)
    (else
      (bind _asbp_game_state (cast `/Game/BluePrints/BP_GameState` (`GameplayStatics.GetGameState`)))
      (bind _can_move (`/Game/BluePrints/BP_GameState.Can Move` _asbp_game_state))
      (if (and (not (`self.IsWander`)) _can_move)
        (`self.Wander`)))))

(event `Deal Damage`
  (params (Damage :type "Float (double-precision)"))
  (if (> (`self.Health`) 0.0)
    (bind _output_get (set `self.Health` (- (`self.Health`) Damage)))
    (if (<= _output_get 0.0)
      (bind _asbp_game_state (cast `/Game/BluePrints/BP_GameState` (`GameplayStatics.GetGameState`)))
      (`/Game/BluePrints/BP_GameState.Kill Robot` _asbp_game_state)
      (`PrimitiveComponent.SetSimulatePhysics` (`self.Mesh`) true)
      (`PrimitiveComponent.SetCollisionEnabled` (`self.Mesh`) "QueryAndPhysics"))))

(event `self.ReceivePointDamage`
  (params (Damage :type "Float (single-precision)") (DamageType :type "DamageType Object Reference") (HitLocation :type "Vector Structure") (HitNormal :type "Vector Structure") (HitComponent :type "PrimitiveComponent Object Reference") (BoneName :type Name) (ShotFromDirection :type "Vector Structure") (InstigatedBy :type "Controller Object Reference") (DamageCauser :type "Actor Object Reference") (HitInfo :type "HitResult Structure (by ref)"))
  (`parent.ReceivePointDamage` Damage DamageType HitLocation HitNormal HitComponent BoneName ShotFromDirection InstigatedBy DamageCauser HitInfo)
  (`self.Deal Damage` Damage)
  (bind _asbp_default_gun_damage (cast `/Game/Weapons/BluePrints/BP_DefaultGunDamage` DamageType))
  (`CharacterMovementComponent.AddImpulse` (`self.CharacterMovement`) (* (`KismetMathLibrary.Normal` ShotFromDirection) (`DamageType.DamageImpulse` _asbp_default_gun_damage)) false))

(event `self.ReceiveRadialDamage`
  (params (DamageReceived :type "Float (single-precision)") (DamageType :type "DamageType Object Reference") (Origin :type "Vector Structure") (HitInfo :type "HitResult Structure (by ref)") (InstigatedBy :type "Controller Object Reference") (DamageCauser :type "Actor Object Reference"))
  (`parent.ReceiveRadialDamage` DamageReceived DamageType Origin HitInfo InstigatedBy DamageCauser)
  (`self.Deal Damage` DamageReceived)
  (bind _asbp_default_grenade_damage (cast `/Game/Weapons/BluePrints/BP_DefaultGrenadeDamage` DamageType))
  (`CharacterMovementComponent.AddImpulse` (`self.CharacterMovement`) (* (`KismetMathLibrary.Normal` (- (`self.K2_GetActorLocation`) Origin)) (`DamageType.DamageImpulse` _asbp_default_grenade_damage)) false))

(fn `UserConstructionScript`
  (`parent.UserConstructionScript`))