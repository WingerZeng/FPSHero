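; BP_ButtonObstacle is a toggle button that switches the game's obstacle state on or off.
; It inherits its checked-state handling from a parent class, calling the parent on BeginPlay and on each state change.
; On a state change, it casts the game state to BP_GameState and passes IsChecked to SetObstacleState.
; The nodes for setting an ON/OFF text label are disconnected, leaving the final branch empty.
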(event `self.ReceiveBeginPlay`
  (`parent.StateChanged` (`self.IsChecked`)))

(event `self.StateChanged`
  (params (isChecked :type Boolean))
  (`parent.StateChanged` isChecked)
  (bind _asbp_game_state (cast `/Game/BluePrints/BP_GameState` (`GameplayStatics.GetGameState`)))
  (`/Game/BluePrints/BP_GameState.Set Obstacle State` _asbp_game_state isChecked)
  (if isChecked
    _))

(fn `UserConstructionScript`
  (`parent.UserConstructionScript`))